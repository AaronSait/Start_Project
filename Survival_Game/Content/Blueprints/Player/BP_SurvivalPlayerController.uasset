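; Player controller for the survival game that owns and switches the player's UI: HUD, notification stack, inventory, loot menu and death screen.
; Most widgets are created lazily and cached, while the loot menu is rebuilt on each show.
; The inventory input toggles its widget with UI-only focus, and the in-game and death screens clear other widgets first.
; Events forward notifications and hit-marker animations, with X firing a test notification.
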(event Custom|CreateNotifcationUI
  (Utilities|IsValid (Variables|Default|GetNotificationWidget)
    (:Is%20Valid
      _)
    (:Is%20Not%20Valid
      (bind _returnvalue (UserInterface|CreateWidget "/Game/UserInterface/Widgets/WBP_NotificationStack.WBP_NotificationStack_C"))
      (bind _output_get (Variables|Default|SetNotificationWidget _returnvalue))))
  (UserInterface|Viewport|AddtoViewport (Variables|Default|GetNotificationWidget) 0))

(event Custom|AddInGameUI
  (Utilities|IsValid (Variables|Default|GetInGameWidget)
    (:Is%20Valid
      _)
    (:Is%20Not%20Valid
      (bind _returnvalue (UserInterface|CreateWidget "/Game/UserInterface/Widgets/WBP_MainHUD.WBP_MainHUD_C"))
      (bind _output_get (Variables|Default|SetInGameWidget _returnvalue))))
  (UserInterface|Viewport|AddtoViewport (Variables|Default|GetInGameWidget) 0))

(event EventBeginPlay)

(event EventTick
  (params (DeltaSeconds :type Float%20%28single-precision%29)))

(event EventShowIngameUI
  (Viewport|RemoveAllWidgets)
  (CallFunction|CreateNotifcationUI)
  (CallFunction|AddinGameUI))

(event EventShowNotification
  (params (message :type Text%20%28by%20ref%29))
  (Utilities|IsValid (Variables|Default|GetNotificationWidget)
    (:Is%20Valid
      (Default|AddNotification (Variables|Default|GetNotificationWidget) message))))

(event EventShowLootMenu
  (params (lootSource :type Inventory%20Component%20Object%20Reference))
  (bind _returnvalue (UserInterface|CreateWidget "/Game/UserInterface/Widgets/WBP_LootMenu.WBP_LootMenu_C"))
  (bind _output_get (Variables|Default|SetLootMenuWidget _returnvalue))
  (UserInterface|Viewport|AddtoViewport _output_get 0))

(event EventHideLootMenu
  (Widget|RemovefromParent (Variables|Default|GetLootMenuWidget)))

(event EventShowDeathMenu
  (Viewport|RemoveAllWidgets)
  (Utilities|IsValid (Variables|Default|GetDeathScreenWidget)
    (:Is%20Valid
      _)
    (:Is%20Not%20Valid
      (bind _returnvalue (UserInterface|CreateWidget "/Game/UserInterface/Widgets/WBP_DeathScreen.WBP_DeathScreen_C"))
      (Variables|Default|SetDeathScreenWidget _returnvalue)))
  (UserInterface|Viewport|AddtoViewport (Variables|Default|GetDeathScreenWidget) 0))

(event EventOnHitPlayer
  (bind _ingamewidget (Variables|Default|GetInGameWidget))
  (Utilities|IsValid _ingamewidget
    (:Is%20Valid
      (UserInterface|Animation|PlayAnimation _ingamewidget (Variables|/Game/UserInterface/Widgets/WBP_MainHUD.WBP_MainHUD_C|GetHitMarkerAnim _ingamewidget) 0.0 1 "Forward" 1.0 false))))

(event Input|ActionEvents|InputActionOpenInventoy
  (params (Key :type Key%20Structure :default "None"))
  (:Pressed
    (Utilities|IsValid (Variables|Default|GetInventoryWidget)
      (:Is%20Valid
        (if (UserInterface|Viewport|IsinViewport (Variables|Default|GetInventoryWidget))
          (Default|CloseInventory (Variables|Default|GetInventoryWidget))
          (else
            (Utilities|IsValid 0
              (:Is%20Valid
                _)
              (:Is%20Not%20Valid
                (bind _returnvalue (UserInterface|CreateWidget "/Game/UserInterface/Widgets/WBP_Inventory.WBP_Inventory_C" :!label _label))
                (bind _output_get (Variables|Default|SetInventoryWidget _returnvalue))))
            (UserInterface|Viewport|AddtoViewport (Variables|Default|GetInventoryWidget) 0)
            (Variables|Default|SetbShowMouseCursor true)
            (Input|SetInputModeUIOnly self (Variables|Default|GetInventoryWidget) "DoNotLock"))))
      (:Is%20Not%20Valid
        (goto _label)))))

(event Input|KeyboardEvents|X
  (params (Key :type Key%20Structure :default "None"))
  (:Pressed
    (Class|SurvivalPlayerController|ShowNotification (Utilities|Text|MakeLiteralText "Has This Worked"))))

(fn ConstructionScript)